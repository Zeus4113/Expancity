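; BP_Office is an office building, a child Blueprint that specializes a parent building's upgrade behavior.
; UpgradeBuilding runs only if not already upgraded, finds BP_Money_Manager and checks that its current pot covers the upgrade cost.
; It then deducts the cost, sets new worker space, amenity happiness and operating cost values, and calls the parent upgrade.
; The construction script only calls the parent, and the event graph is unused.
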(event EventBeginPlay)

(event Collision|EventActorBeginOverlap
  (params (OtherActor :type Actor%20Object%20Reference)))

(event EventTick
  (params (DeltaSeconds :type Float%20%28single-precision%29)))

(fn ConstructionScript
  (|CallParentFunction))

(fn UpgradeBuilding
  (if (not (Variables|Default|GetisUpgraded))
    (bind _returnvalue (Actor|GetActorOfClass "/Game/Game_Logic/BP_Money_Manager.BP_Money_Manager_C"))
    (if (>= (Variables|/Game/Game_Logic/BP_Money_Manager.BP_Money_Manager_C|GetCurrent%20Pot _returnvalue) (Variables|Default|GetUpgrade%20Cost))
      (Default|AddtoPot _returnvalue (* (Variables|Default|GetUpgrade%20Cost) -1))
      (Variables|Default|SetWorker%20Space 16)
      (Variables|Default|SetAmenity%20Happiness 0.0)
      (Variables|Default|SetOperating%20Cost 400)
      (|CallParentFunction))))