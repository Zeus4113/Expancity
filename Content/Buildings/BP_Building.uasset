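; BP_Building is a grid building that tracks and marks the BP_GridPoint actors under its Base component.
; The construction script derives building width and height from Base's rounded world scale.
; CheckOverlap gathers overlapping points, marks them occupied by the building and prints debug output.
; SetReferences and ClearReferences both run CheckOverlap first, then respectively occupy or clear each point, with ClearReferences taking a destroyed-actor parameter.
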(event Custom|Clear%20References
  (params (DestroyedActor :type Actor%20Object%20Reference))
  (CallFunction|CheckOverlap)
  (for _array_element (Variables|Default|GetOverlappedPoints)
    (bind _asbp_grid_point (Utilities|Casting|CastToBP_GridPoint _array_element))
    (Default|SetPointCleared _asbp_grid_point)))

(event Custom|Set%20References
  (CallFunction|CheckOverlap)
  (for _array_element (Variables|Default|GetOverlappedPoints)
    (bind _asbp_grid_point (Utilities|Casting|CastToBP_GridPoint _array_element))
    (Default|SetPointOccupied _asbp_grid_point self)))

(fn ConstructionScript
  (bind _base (Variables|Default|GetBase))
  (bind _returnvalue (Transformation|GetWorldScale _base))
  (Variables|Default|SetBuilding%20Width (Math|Float|Round (.x _returnvalue)))
  (Variables|Default|SetBuilding%20Height (Math|Float|Round (.y _returnvalue))))

(fn CheckOverlap
  (Development|PrintString "Checking")
  (bind _output_get (Variables|Default|SetOverlappedPoints (Collision|GetOverlappingActors (Variables|Default|GetBase) "/Game/Grid/BP_GridPoint.BP_GridPoint_C" :!class /Script/Engine.PrimitiveComponent)))
  (for _array_element _output_get
    (bind _asbp_grid_point (Utilities|Casting|CastToBP_GridPoint _array_element))
    (Default|SetPointOccupied _asbp_grid_point self))
  (Development|PrintString (Utilities|String|ToString(Integer) (Utilities|Array|Length _output_get))))

(fn GetOverlap
  (bind _output_get (Variables|Default|SetOverlappedPoints (Collision|GetOverlappingActors (Variables|Default|GetBase) "/Game/Grid/BP_GridPoint.BP_GridPoint_C" :!class /Script/Engine.PrimitiveComponent)))
  (return _output_get))