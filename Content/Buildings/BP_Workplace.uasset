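; BP_Workplace is a building Blueprint that tracks the workers assigned to it.
; Add Worker and Remove Worker edit the Workers collection, and Check Space reports whether its count is below WorkerSpace.
; Add Worker does not check capacity itself, the event graph holds only disabled placeholder events, and construction just calls the parent script.
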(event EventBeginPlay)

(event Collision|EventActorBeginOverlap
  (params (OtherActor :type Actor%20Object%20Reference)))

(event EventTick
  (params (DeltaSeconds :type Float%20%28single-precision%29)))

(fn ConstructionScript
  (|CallParentFunction))

(fn AddWorker
  (params (WorkerToAdd :type Char%20Citizen%20Object%20Reference))
  (Utilities|Array|Add (Variables|Default|GetWorkers) WorkerToAdd))

(fn RemoveWorker
  (params (WorkerToRemove :type Char%20Citizen%20Object%20Reference%20%28by%20ref%29))
  (Utilities|Array|RemoveItem (Variables|Default|GetWorkers) WorkerToRemove))

(fn CheckSpace
  (return (< (Utilities|Array|Length (Variables|Default|GetWorkers)) (Variables|Default|GetWorker%20Space))))