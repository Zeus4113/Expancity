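; BP_House is a residential building that houses residents up to a population limit and reports a home happiness score.
; It tracks residents and nearby amenity buildings in arrays, adding each valid amenity's happiness to the building's base value.
; Upgrading, allowed once the BP_Money_Manager pot covers the cost, deducts it, sets new capacity, happiness and operating cost, then calls the parent upgrade.
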(event EventBeginPlay)

(event Collision|EventActorBeginOverlap
  (params (OtherActor :type Actor%20Object%20Reference)))

(event EventTick
  (params (DeltaSeconds :type Float%20%28single-precision%29)))

(fn ConstructionScript
  (|CallParentFunction))

(fn CheckSpace
  (return (< (Utilities|Array|Length (Variables|Default|GetCurrent%20Residents)) (Variables|Default|GetPopulation%20Space))))

(fn AddResident
  (params (ResidentToAdd :type Char%20Citizen%20Object%20Reference))
  (Utilities|Array|Add (Variables|Default|GetCurrent%20Residents) ResidentToAdd))

(fn RemoveResident
  (params (ResidentToRemove :type Char%20Citizen%20Object%20Reference))
  (Utilities|Array|RemoveItem (Variables|Default|GetCurrent%20Residents) ResidentToRemove))

(fn AddAmenity
  (params (New%20Building :type BP%20Workplace%20Object%20Reference%20%28by%20ref%29))
  (bind _nearby_amenities (Variables|Default|GetNearby%20Amenities))
  (Utilities|IsValid New%20Building
    (:Is%20Valid
      (if (not (Utilities|Array|ContainsItem _nearby_amenities New%20Building))
        (Utilities|Array|AddUnique _nearby_amenities New%20Building)))))

(fn RemoveAmenity
  (params (Old%20Building :type BP%20Workplace%20Object%20Reference%20%28by%20ref%29))
  (bind _nearby_amenities (Variables|Default|GetNearby%20Amenities))
  (Utilities|IsValid Old%20Building
    (:Is%20Valid
      (if (Utilities|Array|ContainsItem _nearby_amenities Old%20Building)
        (bind _returnvalue (Utilities|Array|RemoveItem _nearby_amenities Old%20Building))
        (if _returnvalue
          (if (not (> (Utilities|Array|Length _nearby_amenities) 0))
            (Utilities|Array|Clear _nearby_amenities)))))))

(fn GetHomeHappiness
  (LocalVariables|SetHappiness (Variables|Default|GetBuilding%20Happiness))
  (for _array_element (Variables|Default|GetNearby%20Amenities)
    (Utilities|IsValid _array_element
      (:Is%20Valid
        (if (Variables|/Game/Buildings/BP_Workplace.BP_Workplace_C|GetIsAmenity _array_element)
          (bind _amenity_happiness (Default|GetAmenityHappiness _array_element))
          (LocalVariables|SetHappiness (+ _amenity_happiness (LocalVariables|GetHappiness)))))))
  (return (LocalVariables|GetHappiness)))

(fn UpgradeBuilding
  (if (not (Variables|Default|GetisUpgraded))
    (bind _returnvalue (Actor|GetActorOfClass "/Game/Game_Logic/BP_Money_Manager.BP_Money_Manager_C"))
    (if (>= (Variables|/Game/Game_Logic/BP_Money_Manager.BP_Money_Manager_C|GetCurrent%20Pot _returnvalue) (Variables|Default|GetUpgrade%20Cost))
      (Default|AddtoPot _returnvalue (* (Variables|Default|GetUpgrade%20Cost) -1))
      (Variables|Default|SetPopulation%20Space 3)
      (Variables|Default|SetBuilding%20Happiness 3e+01)
      (Variables|Default|SetOperating%20Cost 30)
      (|CallParentFunction))))