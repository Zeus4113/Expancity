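; Grid-placed road tile that visually connects itself to adjacent road tiles.
; On placement, it checks the four cardinal neighbours of each overlapped BP_GridPoint and unhides the North, South, East or West piece where the occupying type matches.
; It then calls InitialiseRoad on those neighbouring tiles, which rerun the same check with IsChecking set, so they update their own connections without propagating further.
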(event Custom|Initialise%20Road
  (Variables|Default|SetIsChecking true)
  (for _array_element (Variables|Default|GetOverlappedPoints)
    (bind _asbp_grid_point (Utilities|Casting|CastToBP_GridPoint _array_element))
    (Utilities|FlowControl|Sequence
      (:then_0
        (bind _asbp_grid_point_2 (Utilities|Casting|CastToBP_GridPoint (Variables|/Game/Grid/BP_GridPoint.BP_GridPoint_C|GetNorthern%20Neighbour _asbp_grid_point)))
        (if (Utilities|Enum|Equal(Enum) (Variables|/Game/Grid/BP_GridPoint.BP_GridPoint_C|GetOccupying%20Type _asbp_grid_point_2) "NewEnumerator0")
          (CallFunction|NorthHidden false)
          (if (not (Variables|Default|GetIsChecking))
            (bind _asbp_road_tile (Utilities|Casting|CastToBP_Road_Tile (Variables|/Game/Grid/BP_GridPoint.BP_GridPoint_C|GetOccupying%20Actor _asbp_grid_point_2)))
            (CallFunction|InitialiseRoad _asbp_road_tile))))
      (:then_1
        (bind _asbp_grid_point_3 (Utilities|Casting|CastToBP_GridPoint (Variables|/Game/Grid/BP_GridPoint.BP_GridPoint_C|GetSouthern%20Neighbour _asbp_grid_point)))
        (if (Utilities|Enum|Equal(Enum) (Variables|/Game/Grid/BP_GridPoint.BP_GridPoint_C|GetOccupying%20Type _asbp_grid_point_3) "NewEnumerator0")
          (CallFunction|SouthHidden false)
          (if (not (Variables|Default|GetIsChecking))
            (bind _asbp_road_tile_2 (Utilities|Casting|CastToBP_Road_Tile (Variables|/Game/Grid/BP_GridPoint.BP_GridPoint_C|GetOccupying%20Actor _asbp_grid_point_3)))
            (CallFunction|InitialiseRoad _asbp_road_tile_2))))
      (:then_2
        (bind _asbp_grid_point_4 (Utilities|Casting|CastToBP_GridPoint (Variables|/Game/Grid/BP_GridPoint.BP_GridPoint_C|GetEastern%20Neighbour _asbp_grid_point)))
        (if (Utilities|Enum|Equal(Enum) (Variables|/Game/Grid/BP_GridPoint.BP_GridPoint_C|GetOccupying%20Type _asbp_grid_point_4) "NewEnumerator0")
          (CallFunction|EastHidden false)
          (if (not (Variables|Default|GetIsChecking))
            (bind _asbp_road_tile_3 (Utilities|Casting|CastToBP_Road_Tile (Variables|/Game/Grid/BP_GridPoint.BP_GridPoint_C|GetOccupying%20Actor _asbp_grid_point_4)))
            (CallFunction|InitialiseRoad _asbp_road_tile_3))))
      (:then_3
        (bind _asbp_grid_point_5 (Utilities|Casting|CastToBP_GridPoint (Variables|/Game/Grid/BP_GridPoint.BP_GridPoint_C|GetWestern%20Neighbour _asbp_grid_point)))
        (if (Utilities|Enum|Equal(Enum) (Variables|/Game/Grid/BP_GridPoint.BP_GridPoint_C|GetOccupying%20Type _asbp_grid_point_5) "NewEnumerator0")
          (CallFunction|WestHidden false)
          (if (not (Variables|Default|GetIsChecking))
            (bind _asbp_road_tile_4 (Utilities|Casting|CastToBP_Road_Tile (Variables|/Game/Grid/BP_GridPoint.BP_GridPoint_C|GetOccupying%20Actor _asbp_grid_point_5)))
            (CallFunction|InitialiseRoad _asbp_road_tile_4)))))))

(event Custom|OnPlaced
  (Variables|Default|SetIsChecking false)
  (for _array_element (Variables|Default|GetOverlappedPoints)
    (bind _asbp_grid_point (Utilities|Casting|CastToBP_GridPoint _array_element))
    (Utilities|FlowControl|Sequence
      (:then_0
        (bind _asbp_grid_point_2 (Utilities|Casting|CastToBP_GridPoint (Variables|/Game/Grid/BP_GridPoint.BP_GridPoint_C|GetNorthern%20Neighbour _asbp_grid_point)))
        (if (Utilities|Enum|Equal(Enum) (Variables|/Game/Grid/BP_GridPoint.BP_GridPoint_C|GetOccupying%20Type _asbp_grid_point_2) "NewEnumerator0")
          (CallFunction|NorthHidden false)
          (if (not (Variables|Default|GetIsChecking))
            (bind _asbp_road_tile (Utilities|Casting|CastToBP_Road_Tile (Variables|/Game/Grid/BP_GridPoint.BP_GridPoint_C|GetOccupying%20Actor _asbp_grid_point_2)))
            (CallFunction|InitialiseRoad _asbp_road_tile))))
      (:then_1
        (bind _asbp_grid_point_3 (Utilities|Casting|CastToBP_GridPoint (Variables|/Game/Grid/BP_GridPoint.BP_GridPoint_C|GetSouthern%20Neighbour _asbp_grid_point)))
        (if (Utilities|Enum|Equal(Enum) (Variables|/Game/Grid/BP_GridPoint.BP_GridPoint_C|GetOccupying%20Type _asbp_grid_point_3) "NewEnumerator0")
          (CallFunction|SouthHidden false)
          (if (not (Variables|Default|GetIsChecking))
            (bind _asbp_road_tile_2 (Utilities|Casting|CastToBP_Road_Tile (Variables|/Game/Grid/BP_GridPoint.BP_GridPoint_C|GetOccupying%20Actor _asbp_grid_point_3)))
            (CallFunction|InitialiseRoad _asbp_road_tile_2))))
      (:then_2
        (bind _asbp_grid_point_4 (Utilities|Casting|CastToBP_GridPoint (Variables|/Game/Grid/BP_GridPoint.BP_GridPoint_C|GetEastern%20Neighbour _asbp_grid_point)))
        (if (Utilities|Enum|Equal(Enum) (Variables|/Game/Grid/BP_GridPoint.BP_GridPoint_C|GetOccupying%20Type _asbp_grid_point_4) "NewEnumerator0")
          (CallFunction|EastHidden false)
          (if (not (Variables|Default|GetIsChecking))
            (bind _asbp_road_tile_3 (Utilities|Casting|CastToBP_Road_Tile (Variables|/Game/Grid/BP_GridPoint.BP_GridPoint_C|GetOccupying%20Actor _asbp_grid_point_4)))
            (CallFunction|InitialiseRoad _asbp_road_tile_3))))
      (:then_3
        (bind _asbp_grid_point_5 (Utilities|Casting|CastToBP_GridPoint (Variables|/Game/Grid/BP_GridPoint.BP_GridPoint_C|GetWestern%20Neighbour _asbp_grid_point)))
        (if (Utilities|Enum|Equal(Enum) (Variables|/Game/Grid/BP_GridPoint.BP_GridPoint_C|GetOccupying%20Type _asbp_grid_point_5) "NewEnumerator0")
          (CallFunction|WestHidden false)
          (if (not (Variables|Default|GetIsChecking))
            (bind _asbp_road_tile_4 (Utilities|Casting|CastToBP_Road_Tile (Variables|/Game/Grid/BP_GridPoint.BP_GridPoint_C|GetOccupying%20Actor _asbp_grid_point_5)))
            (CallFunction|InitialiseRoad _asbp_road_tile_4)))))))

(fn ConstructionScript
  (|CallParentFunction))

(fn NorthHidden
  (params (IsHidden :type Boolean))
  (Development|SetHiddeninGame (Variables|Default|GetNorth) IsHidden false))

(fn SouthHidden
  (params (IsHidden :type Boolean))
  (Development|SetHiddeninGame (Variables|Default|GetSouth) IsHidden false))

(fn EastHidden
  (params (IsHidden :type Boolean))
  (Development|SetHiddeninGame (Variables|Default|GetEast) IsHidden false))

(fn WestHidden
  (params (IsHidden :type Boolean))
  (Development|SetHiddeninGame (Variables|Default|GetWest) IsHidden false))