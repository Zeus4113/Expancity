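; BP_Cinema is a cinema building that acts as an amenity for nearby houses.
; Overlaps with its ParkArea component add the cinema to each BP_House's amenities, and end overlaps remove it.
; Both events act only while the cinema has an AC_Clickable component.
; Construction defers entirely to the parent class.
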(event OnComponentBeginOverlap(ParkArea)
  (params (OverlappedComponent :type Primitive%20Component%20Object%20Reference) (OtherActor :type Actor%20Object%20Reference) (OtherComp :type Primitive%20Component%20Object%20Reference) (OtherBodyIndex :type Integer) (bFromSweep :type Boolean) (SweepResult :type Hit%20Result%20Structure%20%28by%20ref%29))
  (Utilities|IsValid (Actor|GetComponentbyClass self "/Game/Components/AC_Clickable.AC_Clickable_C")
    (:Is%20Valid
      (bind _asbp_house (Utilities|Casting|CastToBP_House OtherActor))
      (Default|AddAmenity _asbp_house self))))

(event OnComponentEndOverlap(ParkArea)
  (params (OverlappedComponent :type Primitive%20Component%20Object%20Reference) (OtherActor :type Actor%20Object%20Reference) (OtherComp :type Primitive%20Component%20Object%20Reference) (OtherBodyIndex :type Integer))
  (Utilities|IsValid (Actor|GetComponentbyClass self "/Game/Components/AC_Clickable.AC_Clickable_C")
    (:Is%20Valid
      (bind _asbp_house (Utilities|Casting|CastToBP_House OtherActor))
      (Default|RemoveAmenity _asbp_house self))))

(fn ConstructionScript
  (|CallParentFunction))