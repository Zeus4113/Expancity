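; Grid point actor for a building placement grid that records which building occupies it and its type.
; On BeginPlay or Initialize, it finds its four cardinal neighbours by offsetting its index in BP_PlacementGrid's flat array by one or GridSize, without row-edge checks.
; Occupying it with a BP_Building stores the building type and turns neighbouring meshes green.
; Clearing resets occupant and type but leaves neighbour materials unchanged.
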(event Custom|Set%20Point%20Cleared
  (Variables|Default|SetOccupying%20Actor 0)
  (Variables|Default|SetOccupying%20Type "NewEnumerator3"))

(event Custom|Set%20Point%20Occupied
  (params (Placed%20Actor :type Actor%20Object%20Reference))
  (bind _output_get (Variables|Default|SetOccupying%20Actor Placed%20Actor))
  (bind _asbp_building (Utilities|Casting|CastToBP_Building _output_get))
  (Variables|Default|SetOccupying%20Type (Variables|/Game/Buildings/BP_Building.BP_Building_C|GetBuilding%20Type _asbp_building))
  (for _array_element (Variables|Default|GetNeighbours)
    (Rendering|Material|SetMaterial (Actor|GetComponentbyClass _array_element "/Script/Engine.StaticMeshComponent") 0 "/Game/Materials/M_Green.M_Green")))

(event Custom|Initialize
  (bind _neighbours (Variables|Default|GetNeighbours))
  (Utilities|Array|Clear (Variables|Default|GetNeighbours))
  (bind _returnvalue (Actor|GetActorOfClass "/Game/BP_PlacementGrid.BP_PlacementGrid_C"))
  (Utilities|IsValid _returnvalue
    (:Is%20Valid
      (Utilities|FlowControl|Sequence
        (:then_0
          (Utilities|IsValid (Utilities|Array|Get(acopy) (Variables|/Game/BP_PlacementGrid.BP_PlacementGrid_C|GetGrid%20Points _returnvalue) (+ (Utilities|Array|FindItem (Variables|/Game/BP_PlacementGrid.BP_PlacementGrid_C|GetGrid%20Points _returnvalue) self) 1))
            (:Is%20Valid
              (bind _output_get (Variables|Default|SetEastern%20Neighbour (Utilities|Array|Get(acopy) (Variables|/Game/BP_PlacementGrid.BP_PlacementGrid_C|GetGrid%20Points _returnvalue) (+ (Utilities|Array|FindItem (Variables|/Game/BP_PlacementGrid.BP_PlacementGrid_C|GetGrid%20Points _returnvalue) self) 1))))
              (Utilities|Array|Add _neighbours _output_get))))
        (:then_1
          (Utilities|IsValid (Utilities|Array|Get(acopy) (Variables|/Game/BP_PlacementGrid.BP_PlacementGrid_C|GetGrid%20Points _returnvalue) (- (Utilities|Array|FindItem (Variables|/Game/BP_PlacementGrid.BP_PlacementGrid_C|GetGrid%20Points _returnvalue) self) 1))
            (:Is%20Valid
              (bind _output_get_2 (Variables|Default|SetWestern%20Neighbour (Utilities|Array|Get(acopy) (Variables|/Game/BP_PlacementGrid.BP_PlacementGrid_C|GetGrid%20Points _returnvalue) (- (Utilities|Array|FindItem (Variables|/Game/BP_PlacementGrid.BP_PlacementGrid_C|GetGrid%20Points _returnvalue) self) 1))))
              (Utilities|Array|Add _neighbours _output_get_2))))
        (:then_2
          (Utilities|IsValid (Utilities|Array|Get(acopy) (Variables|/Game/BP_PlacementGrid.BP_PlacementGrid_C|GetGrid%20Points _returnvalue) (+ (Utilities|Array|FindItem (Variables|/Game/BP_PlacementGrid.BP_PlacementGrid_C|GetGrid%20Points _returnvalue) self) (Variables|/Game/BP_PlacementGrid.BP_PlacementGrid_C|GetGrid%20Size _returnvalue)))
            (:Is%20Valid
              (bind _output_get_3 (Variables|Default|SetNorthern%20Neighbour (Utilities|Array|Get(acopy) (Variables|/Game/BP_PlacementGrid.BP_PlacementGrid_C|GetGrid%20Points _returnvalue) (+ (Utilities|Array|FindItem (Variables|/Game/BP_PlacementGrid.BP_PlacementGrid_C|GetGrid%20Points _returnvalue) self) (Variables|/Game/BP_PlacementGrid.BP_PlacementGrid_C|GetGrid%20Size _returnvalue)))))
              (Utilities|Array|Add _neighbours _output_get_3))))
        (:then_3
          (Utilities|IsValid (Utilities|Array|Get(acopy) (Variables|/Game/BP_PlacementGrid.BP_PlacementGrid_C|GetGrid%20Points _returnvalue) (- (Utilities|Array|FindItem (Variables|/Game/BP_PlacementGrid.BP_PlacementGrid_C|GetGrid%20Points _returnvalue) self) (Variables|/Game/BP_PlacementGrid.BP_PlacementGrid_C|GetGrid%20Size _returnvalue)))
            (:Is%20Valid
              (bind _output_get_4 (Variables|Default|SetSouthern%20Neighbour (Utilities|Array|Get(acopy) (Variables|/Game/BP_PlacementGrid.BP_PlacementGrid_C|GetGrid%20Points _returnvalue) (- (Utilities|Array|FindItem (Variables|/Game/BP_PlacementGrid.BP_PlacementGrid_C|GetGrid%20Points _returnvalue) self) (Variables|/Game/BP_PlacementGrid.BP_PlacementGrid_C|GetGrid%20Size _returnvalue)))))
              (Utilities|Array|Add _neighbours _output_get_4))))))))

(event EventBeginPlay
  (bind _neighbours (Variables|Default|GetNeighbours))
  (Utilities|Array|Clear (Variables|Default|GetNeighbours))
  (bind _returnvalue (Actor|GetActorOfClass "/Game/BP_PlacementGrid.BP_PlacementGrid_C"))
  (Utilities|IsValid _returnvalue
    (:Is%20Valid
      (Utilities|FlowControl|Sequence
        (:then_0
          (Utilities|IsValid (Utilities|Array|Get(acopy) (Variables|/Game/BP_PlacementGrid.BP_PlacementGrid_C|GetGrid%20Points _returnvalue) (+ (Utilities|Array|FindItem (Variables|/Game/BP_PlacementGrid.BP_PlacementGrid_C|GetGrid%20Points _returnvalue) self) 1))
            (:Is%20Valid
              (bind _output_get (Variables|Default|SetEastern%20Neighbour (Utilities|Array|Get(acopy) (Variables|/Game/BP_PlacementGrid.BP_PlacementGrid_C|GetGrid%20Points _returnvalue) (+ (Utilities|Array|FindItem (Variables|/Game/BP_PlacementGrid.BP_PlacementGrid_C|GetGrid%20Points _returnvalue) self) 1))))
              (Utilities|Array|Add _neighbours _output_get))))
        (:then_1
          (Utilities|IsValid (Utilities|Array|Get(acopy) (Variables|/Game/BP_PlacementGrid.BP_PlacementGrid_C|GetGrid%20Points _returnvalue) (- (Utilities|Array|FindItem (Variables|/Game/BP_PlacementGrid.BP_PlacementGrid_C|GetGrid%20Points _returnvalue) self) 1))
            (:Is%20Valid
              (bind _output_get_2 (Variables|Default|SetWestern%20Neighbour (Utilities|Array|Get(acopy) (Variables|/Game/BP_PlacementGrid.BP_PlacementGrid_C|GetGrid%20Points _returnvalue) (- (Utilities|Array|FindItem (Variables|/Game/BP_PlacementGrid.BP_PlacementGrid_C|GetGrid%20Points _returnvalue) self) 1))))
              (Utilities|Array|Add _neighbours _output_get_2))))
        (:then_2
          (Utilities|IsValid (Utilities|Array|Get(acopy) (Variables|/Game/BP_PlacementGrid.BP_PlacementGrid_C|GetGrid%20Points _returnvalue) (+ (Utilities|Array|FindItem (Variables|/Game/BP_PlacementGrid.BP_PlacementGrid_C|GetGrid%20Points _returnvalue) self) (Variables|/Game/BP_PlacementGrid.BP_PlacementGrid_C|GetGrid%20Size _returnvalue)))
            (:Is%20Valid
              (bind _output_get_3 (Variables|Default|SetNorthern%20Neighbour (Utilities|Array|Get(acopy) (Variables|/Game/BP_PlacementGrid.BP_PlacementGrid_C|GetGrid%20Points _returnvalue) (+ (Utilities|Array|FindItem (Variables|/Game/BP_PlacementGrid.BP_PlacementGrid_C|GetGrid%20Points _returnvalue) self) (Variables|/Game/BP_PlacementGrid.BP_PlacementGrid_C|GetGrid%20Size _returnvalue)))))
              (Utilities|Array|Add _neighbours _output_get_3))))
        (:then_3
          (Utilities|IsValid (Utilities|Array|Get(acopy) (Variables|/Game/BP_PlacementGrid.BP_PlacementGrid_C|GetGrid%20Points _returnvalue) (- (Utilities|Array|FindItem (Variables|/Game/BP_PlacementGrid.BP_PlacementGrid_C|GetGrid%20Points _returnvalue) self) (Variables|/Game/BP_PlacementGrid.BP_PlacementGrid_C|GetGrid%20Size _returnvalue)))
            (:Is%20Valid
              (bind _output_get_4 (Variables|Default|SetSouthern%20Neighbour (Utilities|Array|Get(acopy) (Variables|/Game/BP_PlacementGrid.BP_PlacementGrid_C|GetGrid%20Points _returnvalue) (- (Utilities|Array|FindItem (Variables|/Game/BP_PlacementGrid.BP_PlacementGrid_C|GetGrid%20Points _returnvalue) self) (Variables|/Game/BP_PlacementGrid.BP_PlacementGrid_C|GetGrid%20Size _returnvalue)))))
              (Utilities|Array|Add _neighbours _output_get_4))))))))

(fn ConstructionScript)