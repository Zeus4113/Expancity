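; Day/night manager that runs an accelerated in-game clock and rotates the directional light to match.
; Once BeginDay is called, a looping timer advances one minute per tick and turns the light a quarter degree, completing one revolution per game day.
; Each tick broadcasts a zero-padded HH:MM string, while hour rollovers fire work, home and day-start calls.
; SetLightRotation holds only unconnected timeline-based rotation logic.
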(event Custom|Minute%20Passed
  (Utilities|FlowControl|Sequence
    (:then_0
      (CallFunction|UpdateTime))
    (:then_1
      (Class|Actor|AddActorWorldRotation (Variables|Default|GetDirectional%20Light) "0.250000,0.000000,0.000000"))
    (:then_2
      (bind _time_string (CallFunction|CalculateTime (Variables|Default|GetCurrent%20Hours) (Variables|Default|GetCurrent%20Minutes))))
    (:then_3
      (Default|CallTimeUpdated _time_string 0.25))))

(event Custom|Begin%20Day
  (Utilities|Time|SetTimerbyEvent (delegate Custom|Minute%20Passed) 0.05 true))

(event Custom|Initialise
  (Variables|Default|SetCurrent%20Hours 12)
  (Variables|Default|SetCurrent%20Minutes 0))

(fn ConstructionScript)

(fn CalculateTime
  (params (Hours :type Integer) (Minutes :type Integer))
  (bind _returnvalue (Utilities|String|ToString(Integer) Hours))
  (bind _returnvalue_2 (Utilities|String|ToString(Integer) Minutes))
  (bind _returnvalue_3 (>= Minutes 10))
  (if (>= Hours 10)
    (if _returnvalue_3
      (return (Utilities|String|Append _returnvalue ":" _returnvalue_2))
      (else
        (return (Utilities|String|Append _returnvalue ":" "0" _returnvalue_2))))
    (elif _returnvalue_3
      (return (Utilities|String|Append "0" _returnvalue ":" _returnvalue_2))
      (else
        (return (Utilities|String|Append "0" _returnvalue ":" "0" _returnvalue_2))))))

(fn SetLightRotation
  (params (Rotation%20Timeline :type Float%20%28double-precision%29)))

(fn UpdateTime
  (bind _result (Math|Integer|IncrementInt (Variables|Default|GetCurrent%20Minutes))
    (:%20%20
      (if (>= _result 60)
        (Variables|Default|SetCurrent%20Minutes 0)
        (bind _result_2 (Math|Integer|IncrementInt (Variables|Default|GetCurrent%20Hours))
          (:%20%20
            (Utilities|FlowControl|Sequence
              (:then_0
                (if (== _result_2 9)
                  (Default|CallWorkTime)))
              (:then_1
                (if (== _result_2 17)
                  (Default|CallHomeTime)))
              (:then_2
                (if (>= _result_2 24)
                  (Variables|Default|SetCurrent%20Hours 0)
                  (Default|CallDayStart))))))))))