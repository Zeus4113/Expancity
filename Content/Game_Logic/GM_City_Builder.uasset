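; GM_City_Builder is the city builder game mode that boots the game's core systems on BeginPlay.
; It finds the placement grid, day/night, money, building and population manager actors in the level and caches them.
; It then initialises them in dependency order, passing day/night and building managers into money and population and binding the building manager to the grid.
; Finally it initialises the player controller, starts the day and refreshes the grid.
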(event EventBeginPlay
  (Utilities|FlowControl|Sequence
    (:then_0
      (bind _returnvalue (Actor|GetActorOfClass "/Game/Grid/BP_PlacementGrid.BP_PlacementGrid_C"))
      (Variables|Default|SetPlacement%20Grid _returnvalue))
    (:then_1
      (bind _returnvalue_2 (Actor|GetActorOfClass "/Game/Game_Logic/BP_Day_Night_Manager.BP_Day_Night_Manager_C"))
      (Variables|Default|SetDay%20Night%20Manager _returnvalue_2))
    (:then_2
      (bind _returnvalue_3 (Actor|GetActorOfClass "/Game/Game_Logic/BP_Money_Manager.BP_Money_Manager_C"))
      (Variables|Default|SetMoney%20Manager _returnvalue_3))
    (:then_3
      (bind _returnvalue_4 (Actor|GetActorOfClass "/Game/Game_Logic/BP_Building_Manager.BP_Building_Manager_C"))
      (Variables|Default|SetBuilding%20Manager _returnvalue_4))
    (:then_4
      (bind _returnvalue_5 (Actor|GetActorOfClass "/Game/Game_Logic/BP_Population_Manager.BP_Population_Manager_C"))
      (Variables|Default|SetPopulation%20Manager _returnvalue_5))
    (:then_5
      (Utilities|FlowControl|Sequence
        (:then_0
          (Utilities|IsValid (Variables|Default|GetPlacement%20Grid)
            (:Is%20Valid
              (Default|SetupGrid (Variables|Default|GetPlacement%20Grid)))))
        (:then_1
          (Utilities|IsValid (Variables|Default|GetDay%20Night%20Manager)
            (:Is%20Valid
              (Default|Initialise (Variables|Default|GetDay%20Night%20Manager))
              (Utilities|IsValid (Variables|Default|GetBuilding%20Manager)
                (:Is%20Valid
                  (Default|Initialise (Variables|Default|GetBuilding%20Manager))
                  (Utilities|IsValid (Variables|Default|GetMoney%20Manager)
                    (:Is%20Valid
                      (Default|Initialise (Variables|Default|GetMoney%20Manager) (Variables|Default|GetDay%20Night%20Manager) (Variables|Default|GetBuilding%20Manager))
                      (Utilities|IsValid (Variables|Default|GetPopulation%20Manager)
                        (:Is%20Valid
                          (Default|Initialise (Variables|Default|GetPopulation%20Manager) (Variables|Default|GetDay%20Night%20Manager) (Variables|Default|GetBuilding%20Manager))
                          (Default|BindBuildManager (Variables|Default|GetPlacement%20Grid) (Variables|Default|GetBuilding%20Manager)))))))))))
        (:then_2
          (bind _aspc_player (Utilities|Casting|CastToPC_Player (Game|GetPlayerController 0)))
          (Default|Initialise _aspc_player)
          (Default|BeginDay (Variables|Default|GetDay%20Night%20Manager))
          (Default|RefreshGrid (Variables|Default|GetPlacement%20Grid)))))))

(fn ConstructionScript)