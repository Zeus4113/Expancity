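; Population manager that tracks citizens and workers against the capacity of houses and workplaces, broadcasting changes to both counts.
; Building add and remove events from the building manager adjust capacity, unassigning residents or workers when their building is removed.
; At each day start it spawns citizens at the town hall to fill free housing, or destroys homeless citizens when none is free.
; The workforce is rebuilt by scanning citizens for valid work references.
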(event Custom|Initialise
  (params (Day%20Night%20Manager :type BP%20Day%20Night%20Manager%20Object%20Reference) (Building%20Manager :type BP%20Building%20Manager%20Object%20Reference))
  (EventDispatchers|BindEventtoDayStart Day%20Night%20Manager (delegate Custom|Day%20Started))
  (EventDispatchers|BindEventtoBuildingAdded Building%20Manager (delegate Custom|Building%20Added))
  (EventDispatchers|BindEventtoBuildingRemoved Building%20Manager (delegate Custom|Building%20Removed)))

(event Custom|Building%20Added
  (params (Building :type BP%20Building%20Object%20Reference))
  (bind _asbp_house (Utilities|Casting|CastToBP_House Building)
    (:then
      (bind _output_get (Variables|Default|SetPopulation%20Max (+ (Variables|/Game/Buildings/BP_House.BP_House_C|GetPopulation%20Space _asbp_house) (Variables|Default|GetPopulation%20Max))))
      (Default|CallPopulationUpdated (Utilities|Array|Length (Variables|Default|GetCurrent%20Population)) _output_get))
    (:CastFailed
      (bind _asbp_workplace (Utilities|Casting|CastToBP_Workplace Building))
      (bind _output_get_2 (Variables|Default|SetWorker%20Max (+ (Variables|/Game/Buildings/BP_Workplace.BP_Workplace_C|GetWorker%20Space _asbp_workplace) (Variables|Default|GetWorker%20Max))))
      (Default|CallWorkforceUpdated (Utilities|Array|Length (Variables|Default|GetCurrent%20Workers)) _output_get_2)
      (CallFunction|CalculateWorkforce))))

(event Custom|Building%20Removed
  (params (Building :type BP%20Building%20Object%20Reference))
  (bind _current_workers (Variables|Default|GetCurrent%20Workers))
  (bind _asbp_house (Utilities|Casting|CastToBP_House Building)
    (:then
      (for _array_element (Variables|/Game/Buildings/BP_House.BP_House_C|GetCurrent%20Residents _asbp_house)
        (Default|SetHome _array_element))
      (bind _output_get (Variables|Default|SetPopulation%20Max (- (Variables|Default|GetPopulation%20Max) (Variables|/Game/Buildings/BP_House.BP_House_C|GetPopulation%20Space _asbp_house))))
      (Default|CallPopulationUpdated (Utilities|Array|Length (Variables|Default|GetCurrent%20Population)) _output_get))
    (:CastFailed
      (bind _asbp_workplace (Utilities|Casting|CastToBP_Workplace Building))
      (for _array_element_2 (Variables|/Game/Buildings/BP_Workplace.BP_Workplace_C|GetWorkers _asbp_workplace)
        (Utilities|Array|RemoveItem _current_workers _array_element_2)
        (Default|SetWork _array_element_2))
      (bind _output_get_2 (Variables|Default|SetWorker%20Max (- (Variables|Default|GetWorker%20Max) (Variables|/Game/Buildings/BP_Workplace.BP_Workplace_C|GetWorker%20Space _asbp_workplace))))
      (Default|CallWorkforceUpdated (Utilities|Array|Length _current_workers) _output_get_2)
      (CallFunction|CalculateWorkforce))))

(event Custom|Day%20Started
  (CallFunction|SpawnNewCitizens))

(fn ConstructionScript)

(fn SpawnNewCitizens
  (if (> (Variables|Default|GetPopulation%20Max) (Utilities|Array|Length (Variables|Default|GetCurrent%20Population)))
    (bind _returnvalue (Actor|GetActorOfClass "/Game/Buildings/BP_Town_Hall.BP_Town_Hall_C"))
    (for _index (range (Utilities|Array|Length (Variables|Default|GetCurrent%20Population)) (- (Variables|Default|GetPopulation%20Max) 1))
      (bind _returnvalue_2 (Game|SpawnActorfromClass "/Game/Char_Citizen.Char_Citizen_C" (Math|Transform|MakeTransform (.location (Transformation|GetActorTransform _returnvalue)) (.rotation (Transformation|GetActorTransform _returnvalue)) "0.300000,0.300000,0.300000") "AdjustIfPossibleButAlwaysSpawn" "MultiplyWithRoot" 0 0))
      (Utilities|Array|Add (Variables|Default|GetCurrent%20Population) _returnvalue_2)
      (Default|CallPopulationUpdated (Utilities|Array|Length (Variables|Default|GetCurrent%20Population)) (Variables|Default|GetPopulation%20Max))
      (CallFunction|CalculateWorkforce))
    (else
      (Utilities|Array|Clear (LocalVariables|GetHomeless%20Citizens))
      (for _array_element (Variables|Default|GetCurrent%20Population)
        (Utilities|IsValid (Variables|/Game/Char_Citizen.Char_Citizen_C|GetHome%20Ref _array_element)
          (:Is%20Not%20Valid
            (Utilities|Array|Add (LocalVariables|GetHomeless%20Citizens) _array_element))))
      (for _array_element_2 (LocalVariables|GetHomeless%20Citizens)
        (Actor|DestroyActor _array_element_2)
        (Utilities|Array|RemoveItem (Variables|Default|GetCurrent%20Population) _array_element_2))
      (Default|CallPopulationUpdated (Utilities|Array|Length (Variables|Default|GetCurrent%20Population)) (Variables|Default|GetPopulation%20Max))
      (CallFunction|CalculateWorkforce))))

(fn CalculateWorkforce
  (bind _current_workers (Variables|Default|GetCurrent%20Workers))
  (Utilities|Array|Clear (Variables|Default|GetCurrent%20Workers))
  (for _array_element (Variables|Default|GetCurrent%20Population)
    (Utilities|IsValid (Variables|/Game/Char_Citizen.Char_Citizen_C|GetWork%20Ref _array_element)
      (:Is%20Valid
        (Utilities|Array|Add _current_workers _array_element)
        (Default|CallWorkforceUpdated (Utilities|Array|Length _current_workers) (Variables|Default|GetWorker%20Max))))))