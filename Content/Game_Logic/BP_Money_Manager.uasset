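; Money manager that tracks the player's cash pot and the income and costs of placed buildings.
; It binds to building manager events to deduct build costs and recalculate cashflow, where workplaces earn profit per worker and buildings incur operating costs.
; The day-night manager's work-time event starts a short one-shot timer that applies net cashflow to the pot.
; Changes broadcast through a CashFlowUpdated dispatcher.
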(event Custom|UpdateMoney
  (CallFunction|CalculateCashflow (Variables|Default|GetCurrentBuildings))
  (CallFunction|AddtoPot (- (Variables|Default|GetMoney%20In) (Variables|Default|GetMoney%20Out)))
  (CallFunction|UpdateCashWidget))

(event Custom|Initialise
  (params (Day%20Night%20Manager :type BP%20Day%20Night%20Manager%20Object%20Reference) (Building%20Manager :type BP%20Building%20Manager%20Object%20Reference))
  (EventDispatchers|BindEventtoBuildingAdded Building%20Manager (delegate Custom|UpdateCurrentPot))
  (EventDispatchers|BindEventtoBuildingsUpdated Building%20Manager (delegate Custom|CheckBuildingData))
  (EventDispatchers|BindEventtoWorkTime Day%20Night%20Manager (delegate Custom|Start%20Timer))
  (bind _buildings (Default|GetBuildings Building%20Manager))
  (CallFunction|CalculateCashflow _buildings)
  (CallFunction|UpdateCashWidget))

(event Custom|CheckBuildingData
  (params (Buildings :type Array%20of%20BP%20Building%20Object%20References))
  (bind _output_get (Variables|Default|SetCurrentBuildings Buildings))
  (CallFunction|CalculateCashflow _output_get))

(event Custom|UpdateCurrentPot
  (params (Building :type BP%20Building%20Object%20Reference))
  (CallFunction|AddtoPot (* (Variables|/Game/Buildings/BP_Building.BP_Building_C|GetBuild%20Cost Building) -1)))

(event Custom|Start%20Timer
  (Utilities|Time|SetTimerbyEvent (delegate Custom|UpdateMoney) 0.1))

(fn ConstructionScript)

(fn AddtoPot
  (params (Amount :type Integer))
  (Variables|Default|SetCurrent%20Pot (+ Amount (Variables|Default|GetCurrent%20Pot)))
  (CallFunction|UpdateCashWidget))

(fn CalculateCashflow
  (params (Buildings :type Array%20of%20BP%20Building%20Object%20References))
  (Variables|Default|SetMoney%20In 0)
  (Variables|Default|SetMoney%20Out 0)
  (for _array_element Buildings
    (Utilities|FlowControl|Sequence
      (:then_0
        (bind _asbp_workplace (Utilities|Casting|CastToBP_Workplace _array_element))
        (Development|PrintString (Utilities|String|ToString(Integer) (Utilities|Array|Length (Variables|/Game/Buildings/BP_Workplace.BP_Workplace_C|GetWorkers _asbp_workplace))))
        (Variables|Default|SetMoney%20In (+ (* (Utilities|Array|Length (Variables|/Game/Buildings/BP_Workplace.BP_Workplace_C|GetWorkers _asbp_workplace)) (Variables|/Game/Buildings/BP_Building.BP_Building_C|GetBuilding%20Profit _asbp_workplace)) (Variables|Default|GetMoney%20In))))
      (:then_1
        (bind _asbp_building (Utilities|Casting|CastToBP_Building _array_element))
        (Variables|Default|SetMoney%20Out (+ (Variables|/Game/Buildings/BP_Building.BP_Building_C|GetOperating%20Cost _asbp_building) (Variables|Default|GetMoney%20Out))))))
  (CallFunction|UpdateCashWidget))

(fn UpdateCashWidget
  (Default|CallCashFlowUpdated (Variables|Default|GetCurrent%20Pot) (Variables|Default|GetMoney%20In) (Variables|Default|GetMoney%20Out)))