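; Money manager actor that tracks the player's building economy: a current pot plus income and operating costs.
; Adding a building deducts its build cost and adjusts income and upkeep; removing one reverses only the recurring amounts, with no refund.
; On each day start from BP_Day_Night_Manager it adds net income to the pot.
; Every change broadcasts CashFlowUpdated; the per-building recalculation functions are never run.
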(event Custom|UpdateMoney
  (Variables|Default|SetCurrent%20Pot (+ (- (Variables|Default|GetMoney%20In) (Variables|Default|GetMoney%20Out)) (Variables|Default|GetCurrent%20Pot)))
  (CallFunction|UpdateCashFlow))

(event EventBeginPlay
  (bind _returnvalue (Actor|GetActorOfClass "/Game/BP_Day_Night_Manager.BP_Day_Night_Manager_C"))
  (EventDispatchers|BindEventtoDayStart _returnvalue (delegate Custom|UpdateMoney))
  (CallFunction|UpdateCashFlow))

(fn ConstructionScript
  (Variables|Default|SetMoney%20Out 0)
  (Variables|Default|SetMoney%20In 500)
  (Variables|Default|SetCurrent%20Pot 3000))

(fn AddBuilding
  (params (Added%20Building :type BP%20Building%20Object%20Reference))
  (Utilities|Array|Add (Variables|Default|GetBuildings) Added%20Building)
  (Variables|Default|SetCurrent%20Pot (- (Variables|Default|GetCurrent%20Pot) (Variables|/Game/Buildings/BP_Building.BP_Building_C|GetBuild%20Cost Added%20Building)))
  (Variables|Default|SetMoney%20In (+ (Variables|Default|GetMoney%20In) (Variables|/Game/Buildings/BP_Building.BP_Building_C|GetBuilding%20Profit Added%20Building)))
  (Variables|Default|SetMoney%20Out (+ (Variables|Default|GetMoney%20Out) (Variables|/Game/Buildings/BP_Building.BP_Building_C|GetOperating%20Cost Added%20Building)))
  (CallFunction|UpdateCashFlow))

(fn RemoveBuilding
  (params (Removed%20Building :type BP%20Building%20Object%20Reference))
  (Utilities|Array|RemoveItem (Variables|Default|GetBuildings) Removed%20Building)
  (Variables|Default|SetMoney%20Out (- (Variables|Default|GetMoney%20Out) (Variables|/Game/Buildings/BP_Building.BP_Building_C|GetOperating%20Cost Removed%20Building)))
  (Variables|Default|SetMoney%20In (- (Variables|Default|GetMoney%20In) (Variables|/Game/Buildings/BP_Building.BP_Building_C|GetBuilding%20Profit Removed%20Building)))
  (CallFunction|UpdateCashFlow))

(fn CalculateMoneyin
  (for _array_element (Variables|Default|GetBuildings)
    (Variables|Default|SetMoney%20In (+ (Variables|Default|GetMoney%20In) (Variables|/Game/Buildings/BP_Building.BP_Building_C|GetBuilding%20Profit _array_element)))))

(fn CalculateMoneyOut
  (for _array_element (Variables|Default|GetBuildings)
    (Variables|Default|SetMoney%20Out (+ (Variables|Default|GetMoney%20Out) (Variables|/Game/Buildings/BP_Building.BP_Building_C|GetOperating%20Cost _array_element)))))

(fn UpdateCashFlow
  (Default|CallCashFlowUpdated (Variables|Default|GetCurrent%20Pot) (Variables|Default|GetMoney%20In) (Variables|Default|GetMoney%20Out)))