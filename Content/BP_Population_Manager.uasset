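; Population manager that tracks housing capacity and the citizen count, broadcasting updates when they change.
; Building manager events add or subtract each house's population space from the maximum.
; At each day start, it spawns citizens at the Town Hall if capacity exceeds population.
; Otherwise, it goes through the citizens and removes those without a valid home from the population.
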(event Custom|Initialise
  (params (Day%20Night%20Manager :type BP%20Day%20Night%20Manager%20Object%20Reference) (Building%20Manager :type BP%20Building%20Manager%20Object%20Reference))
  (EventDispatchers|BindEventtoDayStart Day%20Night%20Manager (delegate Custom|Day%20Started))
  (EventDispatchers|BindEventtoBuildingAdded Building%20Manager (delegate Custom|Building%20Added))
  (EventDispatchers|BindEventtoBuildingRemoved Building%20Manager (delegate Custom|Building%20Removed)))

(event Custom|Building%20Added
  (params (Building :type BP%20Building%20Object%20Reference))
  (bind _asbp_house (Utilities|Casting|CastToBP_House Building))
  (bind _output_get (Variables|Default|SetPopulation%20Max (+ (Variables|/Game/Buildings/BP_House.BP_House_C|GetPopulation%20Space _asbp_house) (Variables|Default|GetPopulation%20Max))))
  (Default|CallPopulationUpdated (Utilities|Array|Length (Variables|Default|GetCurrent%20Population)) _output_get))

(event Custom|Building%20Removed
  (params (Building :type BP%20Building%20Object%20Reference))
  (bind _asbp_house (Utilities|Casting|CastToBP_House Building))
  (bind _output_get (Variables|Default|SetPopulation%20Max (- (Variables|Default|GetPopulation%20Max) (Variables|/Game/Buildings/BP_House.BP_House_C|GetPopulation%20Space _asbp_house))))
  (Default|CallPopulationUpdated (Utilities|Array|Length (Variables|Default|GetCurrent%20Population)) _output_get))

(event Custom|Day%20Started
  (CallFunction|SpawnNewCitizens))

(fn ConstructionScript)

(fn SpawnNewCitizens
  (bind _current_population (Variables|Default|GetCurrent%20Population))
  (if (> (Variables|Default|GetPopulation%20Max) (Utilities|Array|Length (Variables|Default|GetCurrent%20Population)))
    (bind _returnvalue (Actor|GetActorOfClass "/Game/Buildings/BP_Town_Hall.BP_Town_Hall_C"))
    (for _index (range (Utilities|Array|Length (Variables|Default|GetCurrent%20Population)) (Variables|Default|GetPopulation%20Max))
      (bind _returnvalue_2 (Game|SpawnActorfromClass "/Game/Pawn_Citizen.Pawn_Citizen_C" (Transformation|GetActorTransform _returnvalue) "AdjustIfPossibleButAlwaysSpawn" "MultiplyWithRoot" 0 0))
      (Utilities|Array|Add (Variables|Default|GetCurrent%20Population) _returnvalue_2)
      (Default|CallPopulationUpdated (- (Utilities|Array|Length (Variables|Default|GetCurrent%20Population)) 1) (Variables|Default|GetPopulation%20Max)))
    (else
      (for _array_element _current_population
        (Utilities|IsValid (Variables|/Game/Pawn_Citizen.Pawn_Citizen_C|GetHome%20Ref _array_element)
          (:Is%20Not%20Valid
            (Utilities|Array|RemoveItem _current_population _array_element)
            (Actor|DestroyActor)
            (Default|CallPopulationUpdated (- (Utilities|Array|Length (Variables|Default|GetCurrent%20Population)) 1) (Variables|Default|GetPopulation%20Max))))))))