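; AC_Placeable is an actor component that marks whether its owning actor sits in a valid, unobstructed spot for placement.
; It checks the owner's overlapping actors on BeginPlay and on every begin or end overlap, treating any overlap as invalid.
; Each check caches the validity flag and swaps the first material on the owner's static mesh between valid and invalid versions.
; CheckPlacement exposes the cached flag to callers.
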(event Custom|Overlap%20Triggered
  (params (OverlappedActor :type Actor%20Object%20Reference) (OtherActor :type Actor%20Object%20Reference))
  (CallFunction|UpdateOverlap))

(event EventBeginPlay
  (bind _returnvalue (Components|GetOwner))
  (Collision|BindEventtoOnActorBeginOverlap _returnvalue (delegate Custom|Overlap%20Triggered))
  (Collision|BindEventtoOnActorEndOverlap _returnvalue (delegate Custom|Overlap%20Triggered))
  (CallFunction|UpdateOverlap))

(fn UpdateOverlap
  (bind _returnvalue (Components|GetOwner))
  (bind _returnvalue_2 (Components|GetOwner))
  (bind _overlappingactors (Collision|GetOverlappingActors _returnvalue "/Script/Engine.Actor" :!class /Script/Engine.Actor))
  (bind _returnvalue_3 (Actor|GetComponentbyClass _returnvalue_2 "/Script/Engine.StaticMeshComponent"))
  (bind _returnvalue_4 (Utilities|Array|Length _overlappingactors))
  (bind _returnvalue_5 (> _returnvalue_4 0))
  (Variables|Default|SetIsValidPlacement (not _returnvalue_5))
  (if _returnvalue_5
    (Rendering|Material|SetMaterial _returnvalue_3 0 (Variables|Default|GetInvalidPlacementMaterial))
    (else
      (Rendering|Material|SetMaterial _returnvalue_3 0 (Variables|Default|GetValidPlacementMaterial)))))

(fn CheckPlacement
  (return (Variables|Default|GetIsValidPlacement)))