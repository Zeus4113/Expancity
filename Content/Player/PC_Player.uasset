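; PC_Player is the player controller for what appears to be a building management game, setting up camera input and the on-screen HUD.
; A custom Initialise event adds the camera movement Enhanced Input mapping context, then creates the building button, day/night, cashflow and population widgets.
; BeginPlay is empty, and the code creating the building-selected menu is disconnected.
; A ShowCursor function toggles mouse cursor visibility.
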(event Custom|Initialise
  (bind _self self)
  (Input|AddMappingContext (PlayerController|LocalPlayerSubsystems|GetEnhancedInputLocalPlayerSubsystem) "/Game/Input/IMC_Camera_Movement.IMC_Camera_Movement" 0 "(bIgnoreAllPressedKeysUntilRelease=True,bForceImmediately=False)")
  (bind _returnvalue (UserInterface|CreateWidget "/Game/User_Interface/UI_BuildingButton.UI_BuildingButton_C" _self))
  (UserInterface|Viewport|AddtoPlayerScreen _returnvalue)
  (bind _returnvalue_2 (UserInterface|CreateWidget "/Game/User_Interface/UI_Day_Night.UI_Day_Night_C" _self))
  (UserInterface|Viewport|AddtoPlayerScreen _returnvalue_2)
  (bind _returnvalue_3 (UserInterface|CreateWidget "/Game/User_Interface/UI_Cashflow.UI_Cashflow_C" _self))
  (UserInterface|Viewport|AddtoPlayerScreen _returnvalue_3)
  (bind _returnvalue_4 (UserInterface|CreateWidget "/Game/User_Interface/UI_Population.UI_Population_C"))
  (UserInterface|Viewport|AddtoPlayerScreen _returnvalue_4))

(event EventBeginPlay)

(fn ConstructionScript)

(fn ShowCursor
  (params (isShown :type Boolean))
  (Variables|Default|SetbShowMouseCursor isShown))