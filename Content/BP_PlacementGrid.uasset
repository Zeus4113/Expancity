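; Placement grid actor that spawns a square field of BP_GridPoint actors and snaps building positions to it.
; On BeginPlay it builds the points in world coordinates from GridSize, GridScale and Offset, then initializes each.
; GetClosestPoint linearly searches for the nearest point, returning its reference and a position shifted by GetOffsetAmount.
; That shift adds half a cell per extra unit of building width and height.
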(event EventBeginPlay
  (CallFunction|CreateGrid)
  (for _array_element (Variables|Default|GetGrid%20Points)
    (bind _asbp_grid_point (Utilities|Casting|CastToBP_GridPoint _array_element))
    (Default|Initialize _asbp_grid_point)))

(event Collision|EventActorBeginOverlap
  (params (OtherActor :type Actor%20Object%20Reference)))

(event EventTick
  (params (DeltaSeconds :type Float%20%28single-precision%29)))

(fn ConstructionScript)

(fn CreateGrid
  (bind _grid_size (Variables|Default|GetGrid%20Size))
  (bind _grid_scale (Variables|Default|GetGrid%20Scale))
  (bind _offset (Variables|Default|GetOffset))
  (bind _returnvalue (- _grid_size 1))
  (Utilities|Array|Clear (Variables|Default|GetGrid%20Points))
  (for _index (range 0 _returnvalue)
    (for _index_2 (range 0 _returnvalue)
      (bind _returnvalue_2 (Game|SpawnActorfromClass "/Game/BP_GridPoint.BP_GridPoint_C" (Math|Transform|MakeTransform (Math|Vector|MakeVector (* (+ _index_2 _offset) _grid_scale) (* (+ _index _offset) _grid_scale) 0.0)) "Undefined" "MultiplyWithRoot" 0 0))
      (Utilities|Array|Add (Variables|Default|GetGrid%20Points) _returnvalue_2))))

(fn GetClosestPoint
  (params (CurrentPosition :type Vector) (Building%20Width :type Integer) (Building%20Height :type Integer))
  (bind _grid_points (Variables|Default|GetGrid%20Points))
  (bind _output (Utilities|Array|Get(acopy) _grid_points))
  (bind _returnvalue (Transformation|GetActorLocation _output))
  (LocalVariables|SetClosest%20Distance (Math|Vector|Distance(Vector) CurrentPosition _returnvalue))
  (LocalVariables|SetClosest%20Position _returnvalue)
  (for _array_element (Variables|Default|GetGrid%20Points)
    (if (< (Math|Vector|Distance(Vector) CurrentPosition (Transformation|GetActorLocation _array_element)) (LocalVariables|GetClosest%20Distance))
      (LocalVariables|SetClosest%20Distance (Math|Vector|Distance(Vector) CurrentPosition (Transformation|GetActorLocation _array_element)))
      (LocalVariables|SetClosest%20Position (Transformation|GetActorLocation _array_element))
      (LocalVariables|SetClosest%20Grid%20Ref _array_element)))
  (bind _offset_vector1 (CallFunction|GetOffsetAmount Building%20Width Building%20Height))
  (return (+ _offset_vector1 (LocalVariables|GetClosest%20Position)) (LocalVariables|GetClosest%20Grid%20Ref)))

(fn GetOffsetAmount
  (params (Building%20Width :type Integer) (Building%20Height :type Integer))
  (LocalVariables|SetWidth Building%20Width)
  (LocalVariables|SetHeight Building%20Height)
  (LocalVariables|SetOffset%20Amount 0.0)
  (LocalVariables|SetOffset%20Vector "0, 0, 0")
  (for _index (range 2 (LocalVariables|GetWidth))
    (LocalVariables|SetOffset%20Amount (+ (LocalVariables|GetOffset%20Amount) (/ (Variables|Default|GetGrid%20Scale) 2))))
  (LocalVariables|SetOffset%20Vector (Math|Vector|MakeVector (LocalVariables|GetOffset%20Amount) (.Y (Class|KismetMathLibrary|BreakVector3f (LocalVariables|GetOffset%20Vector))) (.Z (Class|KismetMathLibrary|BreakVector3f (LocalVariables|GetOffset%20Vector)))))
  (LocalVariables|SetOffset%20Amount 0.0)
  (for _index_2 (range 2 (LocalVariables|GetHeight))
    (LocalVariables|SetOffset%20Amount (+ (LocalVariables|GetOffset%20Amount) (/ (Variables|Default|GetGrid%20Scale) 2))))
  (LocalVariables|SetOffset%20Vector (Math|Vector|MakeVector (.X (Class|KismetMathLibrary|BreakVector3f (LocalVariables|GetOffset%20Vector))) (LocalVariables|GetOffset%20Amount) (.Z (Class|KismetMathLibrary|BreakVector3f (LocalVariables|GetOffset%20Vector)))))
  (return (LocalVariables|GetOffset%20Vector)))