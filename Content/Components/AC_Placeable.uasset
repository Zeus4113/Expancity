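; AC_Placeable is a component that validates where a BP_Building can be placed on a grid of BP_GridPoints.
; It rechecks on BeginPlay and on each owner overlap change, requiring all overlapped points to be empty.
; Roads fail when exactly four empty neighbours are counted; buildings need at least one adjacent road.
; The result swaps the owner's static mesh materials between valid and invalid, and CheckPlacement returns it.
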(event Custom|Overlap%20Triggered
  (params (OverlappedActor :type Actor%20Object%20Reference) (OtherActor :type Actor%20Object%20Reference))
  (CallFunction|UpdateOverlap))

(event EventBeginPlay
  (bind _returnvalue (Components|GetOwner))
  (Collision|BindEventtoOnActorBeginOverlap _returnvalue (delegate Custom|Overlap%20Triggered))
  (Collision|BindEventtoOnActorEndOverlap _returnvalue (delegate Custom|Overlap%20Triggered))
  (CallFunction|UpdateOverlap))

(fn UpdateOverlap
  (bind _returnvalue (Components|GetOwner))
  (bind _returnvalue_2 (Actor|GetComponentsByClass _returnvalue "/Script/Engine.StaticMeshComponent"))
  (bind _asbp_building (Utilities|Casting|CastToBP_Building (Components|GetOwner)))
  (bind _output_get (Default|GetOverlap _asbp_building))
  (LocalVariables|SetEmptySpaces 0)
  (for _array_element _output_get
    (bind _asbp_grid_point (Utilities|Casting|CastToBP_GridPoint _array_element))
    (if (Utilities|Enum|Equal(Enum) (Variables|/Game/Grid/BP_GridPoint.BP_GridPoint_C|GetOccupying%20Type _asbp_grid_point) "NewEnumerator3")
      (bind _result (Math|Integer|IncrementInt (LocalVariables|GetEmptySpaces))
        (:%20%20
          (Development|PrintString (Utilities|String|ToString(Integer) _result))))))
  (if (== (LocalVariables|GetEmptySpaces) (Utilities|Array|Length _output_get))
    (switch Utilities|FlowControl|Switch|SwitchonBuilding_Types (Variables|/Game/Buildings/BP_Building.BP_Building_C|GetBuilding%20Type _asbp_building)
      (:NewEnumerator0
        (LocalVariables|SetEmptyNeighbours 0)
        (bind _array_element_2 (Utilities|Array|ForEachLoopwithBreak _output_get)
          (:LoopBody
            (bind _asbp_grid_point_2 (Utilities|Casting|CastToBP_GridPoint _array_element_2))
            (for _array_element_3 (Variables|/Game/Grid/BP_GridPoint.BP_GridPoint_C|GetNeighbours _asbp_grid_point_2)
              (bind _asbp_grid_point_3 (Utilities|Casting|CastToBP_GridPoint _array_element_3))
              (if (Utilities|Enum|Equal(Enum) (Variables|/Game/Grid/BP_GridPoint.BP_GridPoint_C|GetOccupying%20Type _asbp_grid_point_3) "NewEnumerator3")
                (Math|Integer|IncrementInt (LocalVariables|GetEmptyNeighbours)))))
          (:Completed
            (if (== (LocalVariables|GetEmptyNeighbours) 4)
              (Variables|Default|SetIsValidPlacement false :!label _label)
              (for _array_element_4 _returnvalue_2
                (Rendering|Material|SetMaterial _array_element_4 0 (Variables|Default|GetInvalidPlacementMaterial)))
              (else
                (Variables|Default|SetIsValidPlacement true :!label _label_2)
                (for _array_element_5 _returnvalue_2
                  (Rendering|Material|SetMaterial _array_element_5 0 (Variables|Default|GetValidPlacementMaterial))))))))
      (:NewEnumerator1
        (LocalVariables|SetAdjacentRoads 0)
        (bind _array_element_6 (Utilities|Array|ForEachLoopwithBreak _output_get)
          (:LoopBody
            (bind _asbp_grid_point_4 (Utilities|Casting|CastToBP_GridPoint _array_element_6))
            (for _array_element_7 (Variables|/Game/Grid/BP_GridPoint.BP_GridPoint_C|GetNeighbours _asbp_grid_point_4)
              (bind _asbp_grid_point_5 (Utilities|Casting|CastToBP_GridPoint _array_element_7))
              (if (Utilities|Enum|Equal(Enum) (Variables|/Game/Grid/BP_GridPoint.BP_GridPoint_C|GetOccupying%20Type _asbp_grid_point_5) "NewEnumerator0")
                (Math|Integer|IncrementInt (LocalVariables|GetAdjacentRoads)))))
          (:Completed
            (if (> (LocalVariables|GetAdjacentRoads) 0)
              (goto _label_2)
              (else
                (goto _label)))))))
    (else
      (goto _label))))

(fn CheckPlacement
  (return (Variables|Default|GetIsValidPlacement)))