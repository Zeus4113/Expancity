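; AC_Clickable is an actor component that lets its owner toggle a selected state when clicked.
; On BeginPlay it gathers every static mesh component on the owning actor.
; Each OnClicked call flips IsSelected and turns custom depth rendering on or off for those meshes.
; CheckSelected exposes the current selection state to other code.
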(event Custom|On%20Clicked
  (bind _static_meshes (Variables|Default|GetStatic%20Meshes))
  (bind _output_get (Variables|Default|SetIsSelected (not (Variables|Default|GetIsSelected))))
  (if _output_get
    (for _array_element _static_meshes
      (Utilities|IsValid _array_element
        (:Is%20Valid
          (Rendering|SetRenderCustomDepth _array_element true))))
    (else
      (for _array_element_2 _static_meshes
        (Utilities|IsValid _array_element_2
          (:Is%20Valid
            (Rendering|SetRenderCustomDepth _array_element_2 false)))))))

(event EventBeginPlay
  (Utilities|Array|Clear (Variables|Default|GetStatic%20Meshes))
  (Variables|Default|SetStatic%20Meshes (Actor|GetComponentsByClass (Components|GetOwner) "/Script/Engine.StaticMeshComponent")))

(fn CheckSelected
  (return (Variables|Default|GetIsSelected)))