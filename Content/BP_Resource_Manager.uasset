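; Resource manager that tracks the money, power and happiness produced by the game's buildings.
; Adding or removing a building updates the Buildings list, adjusts the total for its resource type and broadcasts ResourceUpdated.
; BeginPlay broadcasts all three starting totals.
; CheckCost deducts affordable costs from money without broadcasting, then returns a comparison against the already reduced total.
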(event EventBeginPlay
  (Default|CallResourceUpdated "NewEnumerator0" (Variables|Default|GetProduced%20Money))
  (Default|CallResourceUpdated "NewEnumerator2" (Variables|Default|GetProduced%20Power))
  (Default|CallResourceUpdated "NewEnumerator1" (Variables|Default|GetProduced%20Happiness)))

(fn ConstructionScript)

(fn AddBuilding
  (params (New%20Building :type BP%20Building%20Object%20Reference))
  (bind _resource_amount (Variables|/Game/Buildings/BP_Building.BP_Building_C|GetResource%20Amount New%20Building))
  (Utilities|Array|Add (Variables|Default|GetBuildings) New%20Building)
  (switch Utilities|FlowControl|Switch|SwitchonResource_Types (Variables|/Game/Buildings/BP_Building.BP_Building_C|GetResource%20Type New%20Building)
    (:NewEnumerator0
      (bind _output_get (Variables|Default|SetProduced%20Money (+ (Variables|Default|GetProduced%20Money) _resource_amount)))
      (Default|CallResourceUpdated "NewEnumerator0" _output_get))
    (:NewEnumerator1
      (bind _output_get_2 (Variables|Default|SetProduced%20Happiness (+ (Variables|Default|GetProduced%20Happiness) _resource_amount)))
      (Default|CallResourceUpdated "NewEnumerator1" _output_get_2))
    (:NewEnumerator2
      (bind _output_get_3 (Variables|Default|SetProduced%20Power (+ (Variables|Default|GetProduced%20Power) _resource_amount)))
      (Default|CallResourceUpdated "NewEnumerator2" _output_get_3))))

(fn RemoveBuilding
  (params (Old%20Building :type BP%20Building%20Object%20Reference))
  (bind _resource_amount (Variables|/Game/Buildings/BP_Building.BP_Building_C|GetResource%20Amount Old%20Building))
  (Utilities|Array|RemoveItem (Variables|Default|GetBuildings) Old%20Building)
  (switch Utilities|FlowControl|Switch|SwitchonResource_Types (Variables|/Game/Buildings/BP_Building.BP_Building_C|GetResource%20Type Old%20Building)
    (:NewEnumerator0
      (bind _output_get (Variables|Default|SetProduced%20Money (- (Variables|Default|GetProduced%20Money) _resource_amount)))
      (Default|CallResourceUpdated "NewEnumerator0" _output_get))
    (:NewEnumerator1
      (bind _output_get_2 (Variables|Default|SetProduced%20Happiness (- (Variables|Default|GetProduced%20Happiness) _resource_amount)))
      (Default|CallResourceUpdated "NewEnumerator1" _output_get_2))
    (:NewEnumerator2
      (bind _output_get_3 (Variables|Default|SetProduced%20Power (- (Variables|Default|GetProduced%20Power) _resource_amount)))
      (Default|CallResourceUpdated "NewEnumerator2" _output_get_3))))

(fn CheckCost
  (params (Amount :type Integer))
  (if (> (Variables|Default|GetProduced%20Money) Amount)
    (Variables|Default|SetProduced%20Money (- (Variables|Default|GetProduced%20Money) Amount))
    (return (> (Variables|Default|GetProduced%20Money) Amount))))