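; BP_Building_Manager keeps the central list of BP_Building actors in the level and notifies listeners when it changes.
; Initialise gathers every placed BP_Building and runs an overlap check on each.
; Add and Remove ignore duplicates or unknown buildings, then fire added or removed and list-updated dispatchers.
; Removal also clears the building's references and destroys the actor.
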(event Custom|Initialise
  (bind _outactors (Actor|GetAllActorsOfClass "/Game/Buildings/BP_Building.BP_Building_C"))
  (bind _output_get (Variables|Default|SetBuildings _outactors))
  (for _array_element _output_get
    (Default|CheckOverlap _array_element)))

(fn ConstructionScript)

(fn AddBuilding
  (params (Added%20Building :type BP%20Building%20Object%20Reference))
  (bind _buildings (Variables|Default|GetBuildings))
  (if (not (Utilities|Array|ContainsItem _buildings Added%20Building))
    (Utilities|Array|Add _buildings Added%20Building)
    (Default|CallBuildingAdded Added%20Building)
    (Default|CallBuildingsUpdated (Variables|Default|GetBuildings))))

(fn RemoveBuilding
  (params (Building%20to%20Remove :type BP%20Building%20Object%20Reference))
  (bind _buildings (Variables|Default|GetBuildings))
  (if (Utilities|Array|ContainsItem _buildings Building%20to%20Remove)
    (Utilities|Array|RemoveItem _buildings Building%20to%20Remove)
    (Default|CallBuildingRemoved Building%20to%20Remove)
    (Default|ClearReferences Building%20to%20Remove)
    (Actor|DestroyActor Building%20to%20Remove)
    (Default|CallBuildingsUpdated (Variables|Default|GetBuildings))))

(fn GetBuildings
  (return (Variables|Default|GetBuildings)))