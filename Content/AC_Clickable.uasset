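; Actor component that gives its owner a toggleable selected state with a visual highlight hook through Custom Depth.
; On BeginPlay it caches a Static Mesh Component found on the owner.
; OnClicked flips the selection flag and switches that mesh's Render Custom Depth to match.
; CheckSelected exposes the current state to other Blueprints.
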(event Custom|On%20Clicked
  (bind _object_mesh (Variables|Default|GetObject%20Mesh))
  (bind _output_get (Variables|Default|SetIsSelected (not (Variables|Default|GetIsSelected))))
  (Utilities|IsValid (Variables|Default|GetObject%20Mesh)
    (:Is%20Valid
      (if _output_get
        (Rendering|SetRenderCustomDepth _object_mesh true)
        (else
          (Rendering|SetRenderCustomDepth _object_mesh false))))))

(event EventBeginPlay
  (bind _returnvalue (Components|GetOwner))
  (bind _returnvalue_2 (Actor|GetComponentbyClass _returnvalue "/Script/Engine.StaticMeshComponent"))
  (Utilities|IsValid _returnvalue_2
    (:Is%20Valid
      (Variables|Default|SetObject%20Mesh _returnvalue_2))))

(fn CheckSelected
  (return (Variables|Default|GetIsSelected)))